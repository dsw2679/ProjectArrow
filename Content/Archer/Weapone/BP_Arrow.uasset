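; BP_Arrow is the archer's arrow projectile, which damages what it hits through the Gameplay Ability System.
; On capsule overlap it skips the shooter and actors tagged Gate.
; For other actors, the shooter's ability system component applies GE_ArrowDamage to the target, sends it a damage-received message, then the arrow destroys itself.
; BeginPlay calls IgnoreActorWhenMoving on the shooter with ShouldIgnore false, so shooter exclusion relies on the overlap check.
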(event `self.ReceiveBeginPlay`
  (`PrimitiveComponent.IgnoreActorWhenMoving` (`self.Capsule`) (`self.ShooterActor`) false))

(event `self.Capsule.OnComponentBeginOverlap`
  (params (OverlappedComponent :type "PrimitiveComponent Object Reference") (OtherActor :type "Actor Object Reference") (OtherComp :type "PrimitiveComponent Object Reference") (OtherBodyIndex :type Integer) (bFromSweep :type Boolean) (SweepResult :type "HitResult Structure (by ref)"))
  (bind _shooteractor (`self.ShooterActor`))
  (if (== OtherActor _shooteractor)
    _
    (elif (not (`self.ActorHasTag` OtherActor "Gate"))
      (`AbilitySystemComponent.BP_ApplyGameplayEffectToTarget` :`self` (`AbilitySystemBlueprintLibrary.GetAbilitySystemComponent` _shooteractor) :`GameplayEffectClass` "/Game/GamePlayEffect/GE_ArrowDamage.GE_ArrowDamage_C" :`Target` (`AbilitySystemBlueprintLibrary.GetAbilitySystemComponent` OtherActor))
      (message `/Game/Monsters/Interface/BPI_CombatMonster.OnDamageReceived` OtherActor)
      (`self.K2_DestroyActor`))))

(fn `UserConstructionScript`)