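; BP_LevelManager is a level manager that builds an endless-style tile map at runtime and spawns chests where monsters die.
; On BeginPlay it chains the initial tiles, placing each at the previous tile's ArrowComponent transform.
; Gameplay message listeners spawn BP_Chest on monster deaths and add a tile when BP_TileBase requests the next one.
; SpawnAndDestroyTileAt tracks active tiles, destroying the oldest once the count exceeds the maximum.
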(event `self.ReceiveBeginPlay`
  (bind (_asynctaskproxy _actualchannel _payload) (`|AsyncAction_ListenForGameplayMessages` (struct :`TagName` "Game.Event.Monster.Death") "/Game/MessageRouter/ST_MonsterDeathLocation.ST_MonsterDeathLocation")
    (:`then`
      (bind _output_get (set `self.NextSpawnTransform` (struct)))
      (for _ (range 1 (+ (`self.InitialTilecCount`) 1))
        (bind _spawnedtile (`self.SpawnAndDestroyTileAt` _output_get))
        (set `self.NextSpawnTransform` (`SceneComponent.K2_GetComponentToWorld` (`self.GetComponentByClass` _spawnedtile "/Script/Engine.ArrowComponent"))))
      ;[0.9583 0.9583 0.9583 0.5] Message from BP_TileBase
      (bind (_asynctaskproxy_2 _actualchannel_2 _payload_2) (`|AsyncAction_ListenForGameplayMessages` (struct :`TagName` "Game.Event.Map.GenerateNext") "/Game/MessageRouter/ST_TileMessage.ST_TileMessage")
        (:`OnMessageReceived`
          (`self.SpawnAndDestroyTileAt` (`.SpawnNextLocation_8_C553A3104307A42AAA365CA800424AA3` (break `/Game/MessageRouter/ST_TileMessage` _payload_2))))))
    (:`OnMessageReceived`
      (`|SpawnActorFromClass` "/Game/Chest/BP_Chest.BP_Chest_C" (`KismetMathLibrary.MakeTransform` (`.DeathLocation_2_1F19382A406108FD82A61D9A560D76FC` (break `/Game/MessageRouter/ST_MonsterDeathLocation` _payload))) "AlwaysSpawn" "MultiplyWithRoot" null null))))

(fn `SpawnAndDestroyTileAt`
  (params (SpawnTransform :type "Transform Structure"))
  (returns (SpawnedTile :type "Actor Object Reference"))
  (bind _activetiles (`self.ActiveTiles`))
  (bind _returnvalue (`|SpawnActorFromClass` (`self.TileClass`) SpawnTransform "AlwaysSpawn" "MultiplyWithRoot" null null))
  (`KismetArrayLibrary.Array_Add` _activetiles _returnvalue)
  (if (> (`KismetArrayLibrary.Array_Length` _activetiles) (`self.MaxActiveTiles`))
    (`self.K2_DestroyActor` (`|GetArrayItem` _activetiles))
    (`KismetArrayLibrary.Array_Remove` (`self.ActiveTiles`)))
  (return _returnvalue))

(fn `UserConstructionScript`)