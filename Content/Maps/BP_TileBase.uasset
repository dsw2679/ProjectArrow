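; Base map tile actor that drives chained map generation and spawns monsters when its trigger box is overlapped.
; It registers as a Game Framework component receiver, and on overlap broadcasts a gameplay message carrying the instigator and the Arrow's transform for the next tile.
; MonsterSpawn then spawns BP_Monster at five points: one random pick from each of three pairs, plus two fixed points.
; A tag-based spawn loop is left unconnected.
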(event `self.ReceiveBeginPlay`
  (`GameFrameworkComponentManager.AddReceiver` (subsystem `GameFrameworkComponentManager`) null true))

(event `self.Box.OnComponentBeginOverlap`
  (params (OverlappedComponent :type "PrimitiveComponent Object Reference") (OtherActor :type "Actor Object Reference") (OtherComp :type "PrimitiveComponent Object Reference") (OtherBodyIndex :type Integer) (bFromSweep :type Boolean) (SweepResult :type "HitResult Structure (by ref)"))
  (`GameplayMessageSubsystem.K2_BroadcastMessage` (subsystem `GameplayMessageSubsystem`) (struct :`TagName` "Game.Event.Map.GenerateNext") (make `/Game/MessageRouter/ST_TileMessage` null OtherActor (`SceneComponent.K2_GetComponentToWorld` (`self.Arrow`))))
  (`KismetArrayLibrary.Array_Clear` (`self.TargetSpawnPoints`))
  (`KismetArrayLibrary.Array_Add` (`self.TargetSpawnPoints`) (select `bool` (`KismetMathLibrary.RandomBool`) :`false` (`self.EnemySpawnPoint2`) :`true` (`self.EnemySpawnPoint1`)))
  (`KismetArrayLibrary.Array_Add` (`self.TargetSpawnPoints`) (select `bool` (`KismetMathLibrary.RandomBool`) :`false` (`self.EnemySpawnPoint4`) :`true` (`self.EnemySpawnPoint3`)))
  (`KismetArrayLibrary.Array_Add` (`self.TargetSpawnPoints`) (select `bool` (`KismetMathLibrary.RandomBool`) :`false` (`self.EnemySpawnPoint6`) :`true` (`self.EnemySpawnPoint5`)))
  (`KismetArrayLibrary.Array_Add` (`self.TargetSpawnPoints`) (`self.EnemySpawnPoint7`))
  (`KismetArrayLibrary.Array_Add` (`self.TargetSpawnPoints`) (`self.EnemySpawnPoint8`))
  (for _array_element (`self.TargetSpawnPoints`)
    (`|SpawnActorFromClass` "/Game/Monsters/BP_Monster.BP_Monster_C" (`SceneComponent.K2_GetComponentToWorld` _array_element) "Undefined" "MultiplyWithRoot" null 0.0 null)))

(fn `UserConstructionScript`)