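; BP_Chest is a pickup that grants a random stat boost: fire rate, projectile count, attack damage, move speed or HP.
; The construction script rolls the type and value, then shows them on a Korean text label.
; On box overlap, it applies a gameplay effect to the actor's ASC via SetByCaller tag, fires OnGatePassed and destroys itself.
; It registers as a GameFrameworkComponentManager receiver on BeginPlay.
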(event `self.ReceiveBeginPlay`
  (`GameFrameworkComponentManager.AddReceiver` (subsystem `GameFrameworkComponentManager`) null true))

(event `self.Box.OnComponentBeginOverlap`
  (params (OverlappedComponent :type "PrimitiveComponent Object Reference") (OtherActor :type "Actor Object Reference") (OtherComp :type "PrimitiveComponent Object Reference") (OtherBodyIndex :type Integer) (bFromSweep :type Boolean) (SweepResult :type "HitResult Structure (by ref)"))
  (bind _asc (message `/Game/ThirdPerson/Blueprints/Interface/BPI_Combat.GetTargetASC` OtherActor))
  (`/Engine/EditorBlueprintResources/StandardMacros.IsValid` _asc
    (:`Is Valid`
      (bind _output_get (set `self.ChestValue` (select `/Game/Chest/E_ChestType` (`self.ChestType`) :`NewEnumerator0` 0.1 :`NewEnumerator1` 1.0 :`NewEnumerator2` 5.0 :`NewEnumerator3` 20.0 :`NewEnumerator4` 30.0)))
      (bind _returnvalue (`AbilitySystemBlueprintLibrary.AssignTagSetByCallerMagnitude` (`AbilitySystemComponent.MakeOutgoingSpec` :`self` _asc :`GameplayEffectClass` (`self.EffectToApply`)) (select `/Game/Chest/E_ChestType` (`self.ChestType`) :`NewEnumerator0` (struct :`TagName` "Game.Event.Chest.FireRate") :`NewEnumerator1` (struct :`TagName` "Game.Event.Chest.ProjectileCount") :`NewEnumerator2` (struct :`TagName` "Game.Event.Chest.Damage") :`NewEnumerator3` (struct :`TagName` "Game.Event.Chest.MoveSpeed") :`NewEnumerator4` (struct :`TagName` "Game.Event.Chest.Health") :!type "GameplayTag Structure") _output_get))
      (`AbilitySystemComponent.BP_ApplyGameplayEffectSpecToTarget` _asc _returnvalue _asc)
      (`self.OnGatePassed`)
      (`self.K2_DestroyActor`))))

(event `UpdateVisuals`
  (`TextRenderComponent.K2_SetText` (`self.TextRender`) (`|FormatText` "{Type}  \n    +{Value}" (select `/Game/Chest/E_ChestType` (`self.ChestType`) :`NewEnumerator0` "공격 속도" :`NewEnumerator1` "화살 개수" :`NewEnumerator2` "  공격력" :`NewEnumerator3` "이동 속도" :`NewEnumerator4` "    체력") (`self.ChestValue`))))

(fn `UserConstructionScript`
  (locals (TempRandomIndex :type Integer))
  (bind _temprandomindex (`local.TempRandomIndex`))
  (set `local.TempRandomIndex` (`KismetMathLibrary.RandomIntegerInRange` 0 4))
  (set `self.ChestType` (select `int` _temprandomindex :`0` "NewEnumerator0" :`1` "NewEnumerator1" :`2` "NewEnumerator2" :`3` "NewEnumerator3" :`4` "NewEnumerator4" :!type "/Game/Chest/E_ChestType Enum"))
  (set `self.ChestValue` (select `int` _temprandomindex :`0` 0.1 :`1` 1.0 :`2` 5.0 :`3` 20.0 :`4` 30.0))
  (`self.UpdateVisuals`))