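; GA_PlayerPassive is a gameplay ability that keeps the player character's HP widget in sync with a gameplay attribute.
; On activation it finds the WBP_UserHP widget through the avatar's HPWidget component and sets it to the current attribute value.
; A repeating WaitForAttributeChanged task then pushes each new value to the widget.
; The ability never ends itself, so the listener keeps running after activation.
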(event `self.K2_ActivateAbility`
  (bind _returnvalue (`self.GetAvatarActorFromActorInfo`))
  (bind _asbp_third_person_character (cast `/Game/ThirdPerson/Blueprints/BP_ThirdPersonCharacter` _returnvalue))
  (bind _aswbp_user_hp (cast `/Game/ThirdPerson/Blueprints/HPWidget/WBP_UserHP` (`WidgetComponent.GetUserWidgetObject` (`/Game/ThirdPerson/Blueprints/BP_ThirdPersonCharacter.HPWidget` _asbp_third_person_character))))
  (`/Game/ThirdPerson/Blueprints/HPWidget/WBP_UserHP.SetHP` _aswbp_user_hp (`.ReturnValue` (`AbilitySystemBlueprintLibrary.GetFloatAttribute` _returnvalue (struct :`AttributeName` "Health" :`Attribute` "/Script/MyArrowProject.BaseAttributeSet:Health" :`AttributeOwner` "/Script/CoreUObject.Class'/Script/MyArrowProject.BaseAttributeSet'"))))
  (bind (_asynctaskproxy _attribute _newvalue) (`AbilityAsync_WaitAttributeChanged.WaitForAttributeChanged` (`self.GetAvatarActorFromActorInfo`) (struct :`AttributeName` "Health" :`Attribute` "/Script/MyArrowProject.BaseAttributeSet:Health" :`AttributeOwner` "/Script/CoreUObject.Class'/Script/MyArrowProject.BaseAttributeSet'"))
    (:`Changed`
      (bind _asbp_third_person_character_2 (cast `/Game/ThirdPerson/Blueprints/BP_ThirdPersonCharacter` (`self.GetAvatarActorFromActorInfo`)))
      (bind _aswbp_user_hp_2 (cast `/Game/ThirdPerson/Blueprints/HPWidget/WBP_UserHP` (`WidgetComponent.GetUserWidgetObject` (`/Game/ThirdPerson/Blueprints/BP_ThirdPersonCharacter.HPWidget` _asbp_third_person_character_2))))
      (`/Game/ThirdPerson/Blueprints/HPWidget/WBP_UserHP.SetHP` _aswbp_user_hp_2 _newvalue))))