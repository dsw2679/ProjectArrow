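; Monster actor on the Gameplay Ability System that sacrifices itself on contact, hitting the overlapped target for its remaining health.
; BeginPlay builds its attribute set, applies the stats effect and registers as a GameFrameworkComponentManager receiver.
; Capsule overlap passes negated health as a SetByCaller magnitude to the target's ASC.
; Damage events fire an HP-changed dispatcher; contact or zero health broadcasts a death-location gameplay message and destroys the actor.
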(event `self.ReceiveBeginPlay`
  (bind _returnvalue (`|GenericCreateObject` "/Script/MyArrowProject.BaseAttributeSet"))
  (bind _output_get (set `self.AttributeSet` _returnvalue))
  (`MyAbilityHelpers.InitAbilityActorInfoForASC` (`self.AbilitySystem`) self self _output_get)
  (`AbilitySystemComponent.BP_ApplyGameplayEffectToSelf` :`self` (`self.AbilitySystem`) :`GameplayEffectClass` "/Game/GamePlayEffect/GE_MonsterStats.GE_MonsterStats_C")
  (`GameFrameworkComponentManager.AddReceiver` (subsystem `GameFrameworkComponentManager`) null true))

(event `self.Capsule.OnComponentBeginOverlap`
  (params (OverlappedComponent :type "PrimitiveComponent Object Reference") (OtherActor :type "Actor Object Reference") (OtherComp :type "PrimitiveComponent Object Reference") (OtherBodyIndex :type Integer) (bFromSweep :type Boolean) (SweepResult :type "HitResult Structure (by ref)"))
  (bind _asc (message `/Game/ThirdPerson/Blueprints/Interface/BPI_Combat.GetTargetASC` OtherActor))
  (`/Engine/EditorBlueprintResources/StandardMacros.IsValid` _asc
    (:`Is Valid`
      (bind _output_get (set `self.MyCurrentHealth` (`.ReturnValue` (`AbilitySystemBlueprintLibrary.GetFloatAttributeFromAbilitySystemComponent` (`self.AbilitySystem`) (struct :`AttributeName` "Health" :`Attribute` "/Script/MyArrowProject.BaseAttributeSet:Health" :`AttributeOwner` "/Script/CoreUObject.Class'/Script/MyArrowProject.BaseAttributeSet'")))))
      (bind _returnvalue (`AbilitySystemComponent.MakeOutgoingSpec` :`self` (`self.AbilitySystem`) :`GameplayEffectClass` "/Game/GamePlayEffect/GE_MonsterDamage.GE_MonsterDamage_C"))
      (bind _returnvalue_2 (* _output_get -1.0))
      (`KismetSystemLibrary.PrintString` (`KismetStringLibrary.Conv_DoubleToString` _returnvalue_2))
      (bind _returnvalue_3 (`AbilitySystemBlueprintLibrary.AssignTagSetByCallerMagnitude` _returnvalue (struct :`TagName` "Game.Event.Monster.Overlap") _returnvalue_2))
      (`AbilitySystemComponent.BP_ApplyGameplayEffectSpecToTarget` (`self.AbilitySystem`) _returnvalue_3 _asc)
      (`GameplayMessageSubsystem.K2_BroadcastMessage` (subsystem `GameplayMessageSubsystem`) (struct :`TagName` "Game.Event.Monster.Death") (make `/Game/MessageRouter/ST_MonsterDeathLocation` (`SceneComponent.K2_GetComponentLocation` (`self.Capsule`))))
      (`self.K2_DestroyActor`))))

(event `OnDamaged`
  (if (<= (`.ReturnValue` (`AbilitySystemBlueprintLibrary.GetFloatAttributeFromAbilitySystemComponent` (`self.AbilitySystem`) (struct :`AttributeName` "Health" :`Attribute` "/Script/MyArrowProject.BaseAttributeSet:Health" :`AttributeOwner` "/Script/CoreUObject.Class'/Script/MyArrowProject.BaseAttributeSet'"))) 0.0)
    (`GameplayMessageSubsystem.K2_BroadcastMessage` (subsystem `GameplayMessageSubsystem`) (struct :`TagName` "Game.Event.Monster.Death") (make `/Game/MessageRouter/ST_MonsterDeathLocation` (`SceneComponent.K2_GetComponentLocation` (`self.Capsule`))))
    (`self.K2_DestroyActor`)))

(event `/Game/Monsters/Interface/BPI_CombatMonster.OnDamageReceived`
  (`self.OnDamaged`)
  (`self.OnHPChangedDispatcher` (`self.MyCurrentHealth`)))

(event `/Game/Monsters/Interface/BPI_OverlapedbyMonster.OverlapMonster`
  (params (NewParam :type "/Game/ThirdPerson/Blueprints/BP_ThirdPersonCharacter Object Reference")))

(fn `MonsterASC`
  (returns (ASC :type "AbilitySystemComponent Object Reference"))
  (return (`self.AbilitySystem`)))

(fn `UserConstructionScript`)